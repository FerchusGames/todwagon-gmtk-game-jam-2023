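; BP_PlayerCar is a player car actor that automatically travels along the spline of a BP_Spline actor found at BeginPlay.
; MoveObject plays a sound, waits briefly, then runs a timeline with play rate scaled by Speed over spline length.
; Each update places the car by distance along the spline, using world-space location but local-space rotation.
; IsSplineCompleted is set when the timeline finishes.
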(event Custom|MoveObject
  (bind _splineref (Variables|Default|GetSplineRef))
  (bind _spline (Variables|/Game/_Main/Ambulance/BP_Spline.BP_Spline_C|GetSpline _splineref))
  (Audio|PlaySoundatLocation "/Game/_Main/FX/SoundCues/SC_CarritoGangster.SC_CarritoGangster" (Transformation|GetActorLocation) "0, 0, 0" 1.0 1.0 0.0 0 0 0 0)
  (Utilities|FlowControl|Delay 1.0)
  (Components|Timeline|SetPlayRate (Variables|Default|GetMoveObjectT) (/ (Variables|Default|GetSpeed) (Spline|GetSplineLength (Variables|/Game/_Main/Ambulance/BP_Spline.BP_Spline_C|GetSpline (Variables|Default|GetSplineRef)))))
  (bind _movetrack (Timeline|MoveObjectT Play)
    (:Update
      (Transformation|SetActorTransform (Math|Transform|MakeTransform (Spline|GetLocationatDistanceAlongSpline _spline (Math|Float|Lerp 0.0 (Spline|GetSplineLength (Variables|/Game/_Main/Ambulance/BP_Spline.BP_Spline_C|GetSpline (Variables|Default|GetSplineRef))) _movetrack) "World") (Spline|GetRotationatDistanceAlongSpline _spline (Math|Float|Lerp 0.0 (Spline|GetSplineLength (Variables|/Game/_Main/Ambulance/BP_Spline.BP_Spline_C|GetSpline (Variables|Default|GetSplineRef))) _movetrack) "Local") "1.000000,1.000000,1.000000")))
    (:Finished
      (Variables|Default|SetisSplineCompleted true))))

(event EventBeginPlay
  (bind _returnvalue (Actor|GetActorOfClass "/Game/_Main/Ambulance/BP_Spline.BP_Spline_C"))
  (bind _output_get (Variables|Default|SetSplineRef _returnvalue))
  (Utilities|IsValid _output_get
    (:Is%20Valid
      (CallFunction|MoveObject))
    (:Is%20Not%20Valid
      (Development|PrintString "No Spline Found"))))

(fn ConstructionScript)