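; BP_Ambulance is an ambulance actor that travels along the first BP_Spline found in the level.
; On BeginPlay, a timeline with play rate scaled by TimeToComplete sets its transform from spline distance, using world-space location but local-space rotation.
; Collider overlaps apply an impulse to the Collider itself, using the spline start's world location as the vector, and print its name.
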(event OnComponentBeginOverlap(Collider)
  (params (OverlappedComponent :type Primitive%20Component%20Object%20Reference) (OtherActor :type Actor%20Object%20Reference) (OtherComp :type Primitive%20Component%20Object%20Reference) (OtherBodyIndex :type Integer) (bFromSweep :type Boolean) (SweepResult :type Hit%20Result%20Structure%20%28by%20ref%29))
  (Physics|AddImpulse OverlappedComponent (Spline|GetLocationatDistanceAlongSpline (Variables|/Game/_Main/Ambulance/BP_Spline.BP_Spline_C|GetSpline (Variables|Default|GetSplineRef)) (Math|Float|Lerp 0.0 (Spline|GetSplineLength (Variables|/Game/_Main/Ambulance/BP_Spline.BP_Spline_C|GetSpline (Variables|Default|GetSplineRef))) 0.0) "World") "None" false)
  (Development|PrintString (Utilities|GetDisplayName OverlappedComponent)))

(event Custom|MoveObject
  (bind _splineref (Variables|Default|GetSplineRef))
  (bind _spline (Variables|/Game/_Main/Ambulance/BP_Spline.BP_Spline_C|GetSpline _splineref))
  (Components|Timeline|SetPlayRate (Variables|Default|GetMoveObjectT) (/ 1.0 (Variables|Default|GetTimeToComplete)))
  (bind _movetrack (Timeline|MoveObjectT Play)
    (:Update
      (Transformation|SetActorTransform (Math|Transform|MakeTransform (Spline|GetLocationatDistanceAlongSpline _spline (Math|Float|Lerp 0.0 (Spline|GetSplineLength (Variables|/Game/_Main/Ambulance/BP_Spline.BP_Spline_C|GetSpline (Variables|Default|GetSplineRef))) _movetrack) "World") (Spline|GetRotationatDistanceAlongSpline _spline (Math|Float|Lerp 0.0 (Spline|GetSplineLength (Variables|/Game/_Main/Ambulance/BP_Spline.BP_Spline_C|GetSpline (Variables|Default|GetSplineRef))) _movetrack) "Local") "1.000000,1.000000,1.000000")))))

(event EventBeginPlay
  (bind _returnvalue (Actor|GetActorOfClass "/Game/_Main/Ambulance/BP_Spline.BP_Spline_C"))
  (bind _output_get (Variables|Default|SetSplineRef _returnvalue))
  (Utilities|IsValid _output_get
    (:Is%20Valid
      (CallFunction|MoveObject))
    (:Is%20Not%20Valid
      (Development|PrintString "Hello"))))

(fn ConstructionScript)