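; BP_Vehicle_Ambulance is an ambulance vehicle Blueprint with simple health tracking that lets it be destroyed by damage.
; BeginPlay runs the parent logic and fills CurrentHealth from MaxHealth.
; AnyDamage subtracts incoming damage, prints the remaining health, and destroys the actor once it reaches zero or below.
; The construction script only calls its parent.
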(event EventBeginPlay
  (|CallParentFunction)
  (Variables|Default|SetCurrent%20Health (Variables|Default|GetMax%20Health)))

(event Collision|EventActorBeginOverlap
  (params (OtherActor :type Actor%20Object%20Reference)))

(event EventTick
  (params (DeltaSeconds :type Float%20%28single-precision%29)))

(event Game|Damage|EventAnyDamage
  (params (Damage :type Float%20%28single-precision%29) (DamageType :type Damage%20Type%20Object%20Reference) (InstigatedBy :type Controller%20Object%20Reference) (DamageCauser :type Actor%20Object%20Reference))
  (bind _output_get (Variables|Default|SetCurrent%20Health (- (Variables|Default|GetCurrent%20Health) Damage)))
  (Development|PrintString (Utilities|String|ToString(Float) _output_get))
  (if (<= (Variables|Default|GetCurrent%20Health) 0.0)
    (Actor|DestroyActor)))

(fn ConstructionScript
  (|CallParentFunction))