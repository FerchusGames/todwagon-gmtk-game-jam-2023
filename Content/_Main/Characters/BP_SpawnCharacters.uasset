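; BP_SpawnCharacters respawns BP_Character actors whenever the player car finishes its spline.
; On BeginPlay it caches the transforms of all placed characters and a reference to the BP_PlayerCar.
; Tick polls the car's IsSplineCompleted flag, then RespawnCharacters clears it and spawns a new character at each saved transform, ignoring collisions and printing each name.
; It does not destroy existing characters before spawning.
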(event EventBeginPlay
  (Utilities|FlowControl|Sequence
    (:then_0
      (bind _outactors (Actor|GetAllActorsOfClass "/Game/_Main/Characters/BP_Character.BP_Character_C"))
      (for (_array_element _array_index) _outactors
        (Utilities|Array|SetArrayElem (Variables|Default|GetCharactersTransform) _array_index (Transformation|GetActorTransform _array_element) true)))
    (:then_1
      (bind _returnvalue (Actor|GetActorOfClass "/Game/_Main/Player/Car/BP_PlayerCar.BP_PlayerCar_C"))
      (Variables|Default|SetCar _returnvalue))))

(event EventTick
  (params (DeltaSeconds :type Float%20%28single-precision%29))
  (if (Variables|/Game/_Main/Player/Car/BP_PlayerCar.BP_PlayerCar_C|GetisSplineCompleted (Variables|Default|GetCar))
    (CallFunction|RespawnCharacters)))

(fn ConstructionScript)

(fn RespawnCharacters
  (Variables|/Game/_Main/Player/Car/BP_PlayerCar.BP_PlayerCar_C|SetisSplineCompleted (Variables|Default|GetCar) false)
  (for _array_element (Variables|Default|GetCharactersTransform)
    (bind _returnvalue (Game|SpawnActorfromClass "/Game/_Main/Characters/BP_Character.BP_Character_C" _array_element "AlwaysSpawn" 0 0))
    (Development|PrintString (Utilities|String|Append (Utilities|GetDisplayName _returnvalue) " has been spawned."))))