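; BP_Character is a character that ragdolls and screams when a BP_Vehicle hits it, and can explode to damage the player.
; The vehicle overlap enables mesh physics, destroys the trigger so it fires once, and plays the scream at world origin.
; StartDestroyTimer and ClearDestroyTimer, uncalled here, arm or cancel a delayed MakeDamage.
; MakeDamage damages the cached CH_Player regardless of distance, plays an explosion sound and destroys the actor.
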(event OnComponentBeginOverlap(PhysicsTrigger)
  (params (OverlappedComponent :type Primitive%20Component%20Object%20Reference) (OtherActor :type Actor%20Object%20Reference) (OtherComp :type Primitive%20Component%20Object%20Reference) (OtherBodyIndex :type Integer) (bFromSweep :type Boolean) (SweepResult :type Hit%20Result%20Structure%20%28by%20ref%29))
  (Utilities|Casting|CastToBP_Vehicle OtherActor)
  (Physics|SetSimulatePhysics (Variables|Default|GetSkeletalMesh) true)
  (Components|DestroyComponent (Variables|Default|GetPhysics%20Trigger))
  (CallFunction|PlayAAAAHSound))

(event Custom|StartDestroyTimer
  (bind _returnvalue (Utilities|Time|SetTimerbyFunctionName 0 "MakeDamage" 3.0)))

(event Custom|ClearDestroyTimer
  (Utilities|Time|ClearandInvalidateTimerbyHandle (stale Custom|StartDestroyTimer _returnvalue)))

(event EventBeginPlay
  (bind _asch_player (Utilities|Casting|CastToCH_Player (Game|GetPlayerCharacter 0))
    (:then
      (Variables|Default|SetPlayerReference _asch_player))
    (:CastFailed
      (Development|PrintString "Hello"))))

(event Collision|EventActorBeginOverlap
  (params (OtherActor :type Actor%20Object%20Reference)))

(event EventTick
  (params (DeltaSeconds :type Float%20%28single-precision%29)))

(fn ConstructionScript)

(fn MakeDamage
  (Game|Damage|ApplyDamage (Variables|Default|GetPlayerReference) 7.0 0 0)
  (Audio|PlaySoundatLocation "/Game/_Main/FX/SoundCues/SC_Explosion.SC_Explosion" (Transformation|GetActorLocation) "0, 0, 0" 1.0 1.0 0.0 0 0 0 0)
  (Actor|DestroyActor))

(fn PlayAAAAHSound
  (Audio|PlaySoundatLocation "/Game/_Main/FX/SoundCues/SC_Scream.SC_Scream" "0, 0, 0" "0, 0, 0" 1.0 1.0 0.0 0 0 0 0))